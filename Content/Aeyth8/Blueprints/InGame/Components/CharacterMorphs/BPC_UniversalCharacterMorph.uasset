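; BPC_UniversalCharacterMorph is a component that turns a player who bumps into its owning actor into that actor's character.
; On BeginPlay it binds to the owner's OnActorHit event.
; On a hit, it reads the owner's character ID and checks that the other actor is a player-controlled pawn.
; The swap itself runs as an AJBExecInternal SwapCharacter console command, built with that ID and executed for that player's controller.
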(event Custom|EventMorphHit
  (params (SelfActor :type Actor%20Object%20Reference) (OtherActor :type Actor%20Object%20Reference) (NormalImpulse :type Vector) (Hit :type Hit%20Result%20Structure%20%28by%20ref%29))
  (bind _characterid (CallFunction|GetCharacterIdfromActor SelfActor))
  (bind _aspawn (Utilities|Casting|CastToPawn OtherActor))
  (if (Class|Controller|IsPlayerController (Pawn|GetController _aspawn))
    (bind _asplayer_controller (Utilities|Casting|CastToPlayerController (Pawn|GetController _aspawn)))
    (Development|ExecuteConsoleCommand (Utilities|String|Append "AJBExecInternal SwapCharacter " (Utilities|String|ToString(Byte) _characterid)) _asplayer_controller)))

(event EventBeginPlay
  (Collision|BindEventtoOnActorHit (Components|GetOwner) (delegate Custom|EventMorphHit)))

(event EventTick
  (params (DeltaSeconds :type Float%20%28single-precision%29)))