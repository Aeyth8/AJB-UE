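; Blueprint function library of global helpers for hosting, admin, character changes and post-process filter lookup.
; ExecInternal functions wrap AJBExecInternal console commands on player 0, with Host appending URL-style options for area, NPCs, mode and passwords.
; GetPostProcessingFilter searches the controller's child actors for BP_PPV_VSFilter, optionally summoning it by console command and searching again.
; TrySwapCharacter variants use CharacterNo's OnRep or a debug call; SetupForceInvisibleAllWidgetsFlag is an empty stub.
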(fn GetPostProcessingFilter
  (params (bSpawnIfNull :type Boolean))
  (for _array_element (Actor|GetAllChildActors (Game|GetPlayerController 0) true) :!label _label
    (bind _asbp_ppv_vsfilter (Utilities|Casting|CastToBP_PPV_VSFilter _array_element))
    (Utilities|IsValid _asbp_ppv_vsfilter
      (:Is%20Valid
        (LocalVariables|SetPostProcessingFilter _asbp_ppv_vsfilter))))
  (if (Utilities|IsValid (LocalVariables|GetPostProcessingFilter))
    _
    (elif (and bSpawnIfNull (not (LocalVariables|GetbTriedSpawning)))
      (LocalVariables|SetbTriedSpawning true)
      (Development|ExecuteConsoleCommand 0 "summon BP_PPV_VSFilter_C" 0)
      (goto _label)
      (else
        _)))
  (return (LocalVariables|GetPostProcessingFilter)))

(fn SetupForceInvisibleAllWidgetsFlag
  (params (bVisible :type Boolean)))

(fn PrintConsole
  (params (InString :type String))
  (Development|ExecuteConsoleCommand 0 InString 0))

(fn ExecInternalHost
  (params (AreaID :type Byte) (NPCNum :type Integer) (NPCDifficulty :type Byte) (PlayMode :type Byte) (Password :type String) (AdminPassword :type String))
  (bind _returnvalue (Utilities|String|ToString(Byte) AreaID))
  (bind _returnvalue_2 (Utilities|String|ToString(Integer) NPCNum))
  (bind _returnvalue_3 (Utilities|String|Append "?NPCNum=" _returnvalue_2))
  (bind _returnvalue_4 (Utilities|String|Append "AJBExecInternal Host?Area=" _returnvalue _returnvalue_3))
  (LocalVariables|SetbHasNPCs (> NPCNum 0))
  (LocalVariables|SetbHasPassword (> (Utilities|String|Len Password) 0))
  (LocalVariables|SetbHasAdminPassword (> (Utilities|String|Len AdminPassword) 0))
  (Development|ExecuteConsoleCommand 0 (select (LocalVariables|GetbHasAdminPassword) (Utilities|String|Append (select (LocalVariables|GetbHasPassword) (Utilities|String|Append (Utilities|String|Append (select (LocalVariables|GetbHasNPCs) (Utilities|String|Append _returnvalue_4 (Utilities|String|Append "?NPCDifficulty=" (Utilities|String|ToString(Byte) NPCDifficulty))) _returnvalue_4) (Utilities|String|Append "?PlayMode=" (Utilities|String|ToString(Byte) PlayMode))) (Utilities|String|Append "?Password=" Password)) (Utilities|String|Append (select (LocalVariables|GetbHasNPCs) (Utilities|String|Append _returnvalue_4 (Utilities|String|Append "?NPCDifficulty=" (Utilities|String|ToString(Byte) NPCDifficulty))) _returnvalue_4) (Utilities|String|Append "?PlayMode=" (Utilities|String|ToString(Byte) PlayMode)))) (Utilities|String|Append "?AdminPassword=" AdminPassword)) (select (LocalVariables|GetbHasPassword) (Utilities|String|Append (Utilities|String|Append (select (LocalVariables|GetbHasNPCs) (Utilities|String|Append _returnvalue_4 (Utilities|String|Append "?NPCDifficulty=" (Utilities|String|ToString(Byte) NPCDifficulty))) _returnvalue_4) (Utilities|String|Append "?PlayMode=" (Utilities|String|ToString(Byte) PlayMode))) (Utilities|String|Append "?Password=" Password)) (Utilities|String|Append (select (LocalVariables|GetbHasNPCs) (Utilities|String|Append _returnvalue_4 (Utilities|String|Append "?NPCDifficulty=" (Utilities|String|ToString(Byte) NPCDifficulty))) _returnvalue_4) (Utilities|String|Append "?PlayMode=" (Utilities|String|ToString(Byte) PlayMode))))) (Game|GetPlayerController 0)))

(fn ExecInternalChar
  (params (CharacterID :type Integer))
  (Development|ExecuteConsoleCommand 0 (Utilities|String|Append "AJBExecInternal Char " (Utilities|String|ToString(Integer) CharacterID)) (Game|GetPlayerController 0)))

(fn ExecInternalSwapCharacter
  (params (CharacterID :type Integer))
  (Development|ExecuteConsoleCommand 0 (Utilities|String|Append "AJBExecInternal SwapCharacter " (Utilities|String|ToString(Integer) CharacterID)) (Game|GetPlayerController 0)))

(fn ExecInternalGrantAdmin
  (params (PlayerIndex :type Integer))
  (Development|ExecuteConsoleCommand 0 (Utilities|String|Append "AJBExecInternal GrantAdmin " (Utilities|String|ToString(Integer) PlayerIndex)) (Game|GetPlayerController 0)))

(fn ExecInternalRevokeAdmin
  (params (PlayerIndex :type Integer))
  (Development|ExecuteConsoleCommand 0 (Utilities|String|Append "AJBExecInternal RevokeAdmin " (Utilities|String|ToString(Integer) PlayerIndex)) (Game|GetPlayerController 0)))

(fn ExecInternalWinError
  (params (Header :type String) (Body :type String))
  (Development|ExecuteConsoleCommand 0 (Utilities|String|Append "AJBExecInternal WinError " Header "~" Body) (Game|GetPlayerController 0)))

(fn ExecInternalGoldShower
  (Development|ExecuteConsoleCommand 0 "AJBExecInternal GoldShower" (Game|GetPlayerController 0)))

(fn ExecInternalSkipMatchmaking
  (Development|ExecuteConsoleCommand 0 "AJBExecInternal SkipMatchmaking" (Game|GetPlayerController 0)))

(fn ExecInternalAppendOp
  (params (OptionsString :type String))
  (Development|ExecuteConsoleCommand 0 (Utilities|String|Append "AJBExecInternal AppendOp " OptionsString) (Game|GetPlayerController 0)))

(fn TrySwapCharacter
  (params (CharacterID :type Integer))
  (bind _asbp_ajbin_game_player_controller (Utilities|Casting|CastToBP_AJBInGamePlayerController (Game|GetPlayerController 0)))
  (Variables|/Game/AJB/InGame/Core/BP_AJBInGamePlayerController.BP_AJBInGamePlayerController_C|SetCharacterNo _asbp_ajbin_game_player_controller CharacterID)
  (Default|OnRepCharacterNo _asbp_ajbin_game_player_controller))

(fn TrySwapCharacterwithRPC
  (params (CharacterID :type Integer))
  (bind _asbp_ajbin_game_player_controller (Utilities|Casting|CastToBP_AJBInGamePlayerController (Game|GetPlayerController 0)))
  (Default|ROSDebugCharaChange _asbp_ajbin_game_player_controller CharacterID))