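; Server looper actor that restarts a multiplayer session on a random area once the expected players have joined.
; BeginPlay on the server polls every second until the player count matches the NumPlayers URL option.
; Tick then calls Initiate, which unconditionally fires the session-destroy dispatcher and runs an AJBExecInternalHost console command with the current play mode.
; Initiate's non-server branch opens the PendingReconnect map; Tick also prints delta time for debugging.
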(event Custom|EventServerDestroySession
  (|DestroySession (Game|GetPlayerController 0)))

(event EventBeginPlay
  (bind _returnvalue (Game|GetGameMode))
  (EventDispatchers|BindEventtoOnServerDestroySession (delegate Custom|EventServerDestroySession))
  (Variables|Default|SetMyPlayer (Game|GetPlayerController 0))
  (if (Networking|IsServer)
    (bind _returnvalue_2 (Class|GameModeBase|GetNumPlayers _returnvalue :!label _label))
    (Variables|Default|SetCurrentNumPlayers _returnvalue_2)
    (Variables|Default|SetNumPlayersFromFURL (Math|Conversions|ToInteger(Byte) (Class|GameplayStatics|ParseOption (Variables|/Script/Engine.GameModeBase|GetOptionsString _returnvalue) "NumPlayers")))
    (if (!= (Variables|Default|GetCurrentNumPlayers) (Variables|Default|GetNumPlayersFromFURL))
      (Utilities|FlowControl|Delay 1.0)
      (goto _label)
      (else
        (Variables|Default|SetbInitialized true)))))

(event Collision|EventActorBeginOverlap
  (params (OtherActor :type Actor%20Object%20Reference)))

(event EventTick
  (params (DeltaSeconds :type Float%20%28single-precision%29))
  (Development|PrintString (Utilities|String|ToString(Float) DeltaSeconds) true true "(R=0.000000,G=0.660000,B=1.000000,A=1.000000)" 0.1)
  (if (and (Variables|Default|GetbInitialized) (not (Variables|Default|GetbFinished)))
    (CallFunction|Initiate)))

(fn ConstructionScript)

(fn ServerDestroySession
  (if (Networking|IsServer)
    (Default|CallOnServerDestroySession)))

(fn Initiate
  (bind _returnvalue (Game|GetGameMode))
  (if (Networking|IsServer)
    (bind _returnvalue_2 (Class|GameModeBase|GetNumPlayers _returnvalue))
    (Variables|Default|SetCurrentNumPlayers _returnvalue_2)
    (Variables|Default|SetNumPlayersFromFURL (Math|Conversions|ToInteger(Byte) (Class|GameplayStatics|ParseOption (Variables|/Script/Engine.GameModeBase|GetOptionsString _returnvalue) "NumPlayers")))
    (Development|ExecuteConsoleCommand (Utilities|String|Append "NumPlayersFromFURL: " (Utilities|String|ToString(Integer) (Variables|Default|GetNumPlayersFromFURL)) " 
CurrentNumPlayers: " (Utilities|String|ToString(Integer) (Variables|Default|GetCurrentNumPlayers))) (Variables|Default|GetMyPlayer))
    (bind _returnvalue_3 (Class|GameModeBase|GetNumPlayers (Game|GetGameMode)))
    (Variables|Default|SetCurrentNumPlayers _returnvalue_3)
    (if true
      (CallFunction|ServerDestroySession)
      (bind _playmode (CallFunction|GetPlayMode))
      (Development|ExecuteConsoleCommand (Utilities|String|Append "AJBExecInternalHost?Area=" (Utilities|String|ToString(Integer) (Math|Random|RandomIntegerinRange 2 11)) "?Mode=" (Utilities|String|ToString(Byte) _playmode)) (Variables|Default|GetMyPlayer))
      (Variables|Default|SetbFinished true))
    (else
      (Game|OpenLevel(byName) "/Game/Aeyth8/Maps/DedicatedServer/PendingReconnect"))))