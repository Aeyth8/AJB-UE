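; BP_Synchronizer is an actor that mirrors the play mode from server to clients, judging by its ServerReplicated folder and server/client split.
; Every tick, the server copies the current play mode into PlayMode, while clients apply that variable through SetPlayMode.
; Clients also set IsLocalSessionMode on BP_AJBGameInstance, true for the Shop-family modes and false for all others.
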(event EventBeginPlay)

(event Collision|EventActorBeginOverlap
  (params (OtherActor :type Actor%20Object%20Reference)))

(event EventTick
  (params (DeltaSeconds :type Float%20%28single-precision%29))
  (if (Networking|IsServer)
    (bind _playmode (CallFunction|GetPlayMode))
    (Variables|Default|SetPlayMode _playmode)
    (else
      (CallFunction|SetPlayMode (Variables|Default|GetPlayMode))
      (bind _asbp_ajbgame_instance (Utilities|Casting|CastToBP_AJBGameInstance (Game|GetGameInstance)))
      (switch Utilities|FlowControl|Switch|SwitchonPlayMode (Utilities|Enum|ByteToEnumPlayMode (Variables|Default|GetPlayMode))
        (:NewEnumerator0
          (Variables|/Game/AJB/Core/BP_AJBGameInstance.BP_AJBGameInstance_C|SetbIsLocalSessionMode _asbp_ajbgame_instance false :!label _label))
        (:NewEnumerator1
          (goto _label))
        (:NewEnumerator2
          (goto _label))
        (:NewEnumerator3
          ;[1 1 1 1 11] Shop | ShopCompetition | ShopCompetitionPair | ShopExchange
          (Variables|/Game/AJB/Core/BP_AJBGameInstance.BP_AJBGameInstance_C|SetbIsLocalSessionMode _asbp_ajbgame_instance true :!label _label_2))
        (:NewEnumerator4
          (goto _label_2))
        (:NewEnumerator5
          (goto _label))
        (:NewEnumerator6
          (goto _label))
        (:NewEnumerator7
          (goto _label_2))
        (:NewEnumerator8
          (goto _label_2))
        (:NewEnumerator9
          (goto _label))
        (:NewEnumerator10
          (goto _label))
        (:NewEnumerator11
          (goto _label))))))

(fn ConstructionScript)