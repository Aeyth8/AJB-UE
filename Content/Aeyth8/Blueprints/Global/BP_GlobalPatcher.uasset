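; BP_GlobalPatcher is a collection of small, stateless helper functions for text, arrays and maps.
; It converts between strings and text, sets a widget's text from a string, and appends to string or object arrays.
; RemovePlayerAtIndex removes a map entry by looking up the key at the given position in the map's key list.
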(fn SetWidgetText
  (params (TextToEdit :type Text%20Block%20Object%20Reference) (NewText :type String))
  (Rendering|Components|TextRender|SetText TextToEdit (Utilities|Text|ToText(String) NewText)))

(fn TexttoString
  (params (Input :type Text))
  (return (Utilities|String|ToString(Text) Input)))

(fn StringtoText
  (params (input :type String))
  (return (Utilities|Text|ToText(String) input)))

(fn RemovePlayeratIndex
  (params (Index :type Integer) (NewParam :type Map%20of%20Strings%20to%20Structs))
  (bind _keys (Utilities|Map|Keys NewParam))
  (Utilities|Map|Remove NewParam (Utilities|Array|Get(acopy) _keys Index)))

(fn AppendtoFStringArray
  (params (StringArray :type Array%20of%20Strings) (ToAppend :type String))
  (Utilities|Array|Add StringArray ToAppend))

(fn AppendtoObjectArray
  (params (InArray :type Array%20of%20Object%20Object%20References) (ToAppend :type Object%20Object%20Reference))
  (Utilities|Array|Add InArray ToAppend))