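; Actor Blueprint that acts as a one-shot timer, sending a callback to the AJBExecInternal console command after a delay.
; SetCallbackTimer stores the wait time and a callback value split into upper and lower halves, then fires CallbackTimerTick.
; After the Delay, OnBroadcastCallback converts both halves to strings and appends them to the command, using the console as the bridge back to the caller.
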(event Custom|CallbackTimerTick
  (Utilities|FlowControl|Delay (Variables|Default|GetfWaitFor))
  (CallFunction|OnBroadcastCallback (Variables|Default|GetpCallbackUpper) (Variables|Default|GetpCallbackLower)))

(event EventBeginPlay)

(event Collision|EventActorBeginOverlap
  (params (OtherActor :type Actor%20Object%20Reference)))

(event EventTick
  (params (DeltaSeconds :type Float%20%28single-precision%29)))

(fn ConstructionScript)

(fn SetCallbackTimer
  (params (WaitFor :type Float%20%28single-precision%29) (pCallbackUpper :type Integer) (pCallbackLower :type Integer))
  (Variables|Default|SetfWaitFor WaitFor)
  (Variables|Default|SetpCallbackUpper pCallbackUpper)
  (Variables|Default|SetpCallbackLower pCallbackLower)
  (CallFunction|CallbackTimerTick))

(fn OnBroadcastCallback
  (params (pCallbackUpper :type Integer) (pCallbackLower :type Integer))
  (Development|ExecuteConsoleCommand (Utilities|String|Append "AJBExecInternal Callback " (Utilities|String|ToString(Integer) pCallbackUpper) "" (Utilities|String|ToString(Integer) pCallbackLower)) 0))