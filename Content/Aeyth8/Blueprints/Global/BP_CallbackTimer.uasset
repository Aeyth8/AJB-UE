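; BP_CallbackTimer is an actor that counts down registered timers and signals expiry through the console command "AJBExecInternal Callback" plus array index.
; CreateTimer stores a wait time with an address built from two halves as a fake int64.
; InternalTimerTick, driven by Tick or BeginInternalTick's zero-delay loop, accumulates elapsed time and prints debug text.
; Expiry requires truncated elapsed-time text to equal the wait's text, not >=; fired entries remain, flagged.
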(event Custom|EventInternalTick
  (Utilities|FlowControl|Delay 0.0 :!label _label)
  (CallFunction|InternalTimerTick (Utilities|Time|GetWorldDeltaSeconds))
  (goto _label))

(event EventBeginPlay)

(event Collision|EventActorBeginOverlap
  (params (OtherActor :type Actor%20Object%20Reference)))

(event EventTick
  (params (DeltaSeconds :type Float%20%28single-precision%29))
  (CallFunction|InternalTimerTick DeltaSeconds))

(fn ConstructionScript)

(fn CreateTimer
  (params (pUpper :type Integer) (pLower :type Integer) (fWaitFor :type Float%20%28single-precision%29))
  (Utilities|Array|Add (Variables|Default|GetCallbackTimers) (Utilities|Struct|MakeTimerHandlerEntry (Utilities|Struct|MakeFakeInt64 pUpper pLower) fWaitFor 0.0 false)))

(fn InternalTimerTick
  (params (DeltaSeconds :type Float%20%28single-precision%29%20%28by%20ref%29))
  (bind _callbacktimers (Variables|Default|GetCallbackTimers))
  (for (_ _array_index) _callbacktimers
    (bind _output_get (LocalVariables|SetCurrentIndex _array_index))
    (if (not (.bSetForCallback (Utilities|Struct|BreakTimerHandlerEntry (|Copy (Utilities|Array|Get(acopy) _callbacktimers _output_get)))))
      (|SetBy-RefVar (Utilities|Array|Get(acopy) _callbacktimers _output_get) (Utilities|Struct|MakeTimerHandlerEntry (.pAddress (Utilities|Struct|BreakTimerHandlerEntry (|Copy (Utilities|Array|Get(acopy) _callbacktimers _output_get)))) (.fWaitFor (Utilities|Struct|BreakTimerHandlerEntry (|Copy (Utilities|Array|Get(acopy) _callbacktimers _output_get)))) (+ (.fTimeElapsed (Utilities|Struct|BreakTimerHandlerEntry (|Copy (Utilities|Array|Get(acopy) _callbacktimers _output_get)))) DeltaSeconds) (.bSetForCallback (Utilities|Struct|BreakTimerHandlerEntry (|Copy (Utilities|Array|Get(acopy) _callbacktimers _output_get))))))
      (Utilities|FlowControl|Sequence
        (:then_0
          (if (not (.bSetForCallback (Utilities|Struct|BreakTimerHandlerEntry (Utilities|Struct|MakeTimerHandlerEntry (.pAddress (Utilities|Struct|BreakTimerHandlerEntry (|Copy (Utilities|Array|Get(acopy) _callbacktimers _output_get)))) (.fWaitFor (Utilities|Struct|BreakTimerHandlerEntry (|Copy (Utilities|Array|Get(acopy) _callbacktimers _output_get)))) (+ (.fTimeElapsed (Utilities|Struct|BreakTimerHandlerEntry (|Copy (Utilities|Array|Get(acopy) _callbacktimers _output_get)))) DeltaSeconds) (.bSetForCallback (Utilities|Struct|BreakTimerHandlerEntry (|Copy (Utilities|Array|Get(acopy) _callbacktimers _output_get))))))))
            (Development|PrintString (Utilities|String|Append "fWaitFor: " (Utilities|String|ToString(Float) (.fWaitFor (Utilities|Struct|BreakTimerHandlerEntry (Utilities|Struct|MakeTimerHandlerEntry (.pAddress (Utilities|Struct|BreakTimerHandlerEntry (|Copy (Utilities|Array|Get(acopy) _callbacktimers _output_get)))) (.fWaitFor (Utilities|Struct|BreakTimerHandlerEntry (|Copy (Utilities|Array|Get(acopy) _callbacktimers _output_get)))) (+ (.fTimeElapsed (Utilities|Struct|BreakTimerHandlerEntry (|Copy (Utilities|Array|Get(acopy) _callbacktimers _output_get)))) DeltaSeconds) (.bSetForCallback (Utilities|Struct|BreakTimerHandlerEntry (|Copy (Utilities|Array|Get(acopy) _callbacktimers _output_get)))))))) " fTimeElapsed: " (Utilities|String|GetSubstring (Utilities|String|ToString(Float) (.fTimeElapsed (Utilities|Struct|BreakTimerHandlerEntry (Utilities|Struct|MakeTimerHandlerEntry (.pAddress (Utilities|Struct|BreakTimerHandlerEntry (|Copy (Utilities|Array|Get(acopy) _callbacktimers _output_get)))) (.fWaitFor (Utilities|Struct|BreakTimerHandlerEntry (|Copy (Utilities|Array|Get(acopy) _callbacktimers _output_get)))) (+ (.fTimeElapsed (Utilities|Struct|BreakTimerHandlerEntry (|Copy (Utilities|Array|Get(acopy) _callbacktimers _output_get)))) DeltaSeconds) (.bSetForCallback (Utilities|Struct|BreakTimerHandlerEntry (|Copy (Utilities|Array|Get(acopy) _callbacktimers _output_get)))))))) 0 (Utilities|String|Len (Utilities|String|ToString(Float) (.fWaitFor (Utilities|Struct|BreakTimerHandlerEntry (Utilities|Struct|MakeTimerHandlerEntry (.pAddress (Utilities|Struct|BreakTimerHandlerEntry (|Copy (Utilities|Array|Get(acopy) _callbacktimers _output_get)))) (.fWaitFor (Utilities|Struct|BreakTimerHandlerEntry (|Copy (Utilities|Array|Get(acopy) _callbacktimers _output_get)))) (+ (.fTimeElapsed (Utilities|Struct|BreakTimerHandlerEntry (|Copy (Utilities|Array|Get(acopy) _callbacktimers _output_get)))) DeltaSeconds) (.bSetForCallback (Utilities|Struct|BreakTimerHandlerEntry (|Copy (Utilities|Array|Get(acopy) _callbacktimers _output_get))))))))))) true true "(R=0.000000,G=0.660000,B=1.000000,A=1.000000)" 0.1)))
        (:then_1
          (if (and (Utilities|Enum|Equal(Enum) (Utilities|String|ToString(Float) (.fWaitFor (Utilities|Struct|BreakTimerHandlerEntry (Utilities|Struct|MakeTimerHandlerEntry (.pAddress (Utilities|Struct|BreakTimerHandlerEntry (|Copy (Utilities|Array|Get(acopy) _callbacktimers _output_get)))) (.fWaitFor (Utilities|Struct|BreakTimerHandlerEntry (|Copy (Utilities|Array|Get(acopy) _callbacktimers _output_get)))) (+ (.fTimeElapsed (Utilities|Struct|BreakTimerHandlerEntry (|Copy (Utilities|Array|Get(acopy) _callbacktimers _output_get)))) DeltaSeconds) (.bSetForCallback (Utilities|Struct|BreakTimerHandlerEntry (|Copy (Utilities|Array|Get(acopy) _callbacktimers _output_get)))))))) (Utilities|String|GetSubstring (Utilities|String|ToString(Float) (.fTimeElapsed (Utilities|Struct|BreakTimerHandlerEntry (Utilities|Struct|MakeTimerHandlerEntry (.pAddress (Utilities|Struct|BreakTimerHandlerEntry (|Copy (Utilities|Array|Get(acopy) _callbacktimers _output_get)))) (.fWaitFor (Utilities|Struct|BreakTimerHandlerEntry (|Copy (Utilities|Array|Get(acopy) _callbacktimers _output_get)))) (+ (.fTimeElapsed (Utilities|Struct|BreakTimerHandlerEntry (|Copy (Utilities|Array|Get(acopy) _callbacktimers _output_get)))) DeltaSeconds) (.bSetForCallback (Utilities|Struct|BreakTimerHandlerEntry (|Copy (Utilities|Array|Get(acopy) _callbacktimers _output_get)))))))) 0 (Utilities|String|Len (Utilities|String|ToString(Float) (.fWaitFor (Utilities|Struct|BreakTimerHandlerEntry (Utilities|Struct|MakeTimerHandlerEntry (.pAddress (Utilities|Struct|BreakTimerHandlerEntry (|Copy (Utilities|Array|Get(acopy) _callbacktimers _output_get)))) (.fWaitFor (Utilities|Struct|BreakTimerHandlerEntry (|Copy (Utilities|Array|Get(acopy) _callbacktimers _output_get)))) (+ (.fTimeElapsed (Utilities|Struct|BreakTimerHandlerEntry (|Copy (Utilities|Array|Get(acopy) _callbacktimers _output_get)))) DeltaSeconds) (.bSetForCallback (Utilities|Struct|BreakTimerHandlerEntry (|Copy (Utilities|Array|Get(acopy) _callbacktimers _output_get))))))))))) (not (.bSetForCallback (Utilities|Struct|BreakTimerHandlerEntry (Utilities|Struct|MakeTimerHandlerEntry (.pAddress (Utilities|Struct|BreakTimerHandlerEntry (|Copy (Utilities|Array|Get(acopy) _callbacktimers _output_get)))) (.fWaitFor (Utilities|Struct|BreakTimerHandlerEntry (|Copy (Utilities|Array|Get(acopy) _callbacktimers _output_get)))) (+ (.fTimeElapsed (Utilities|Struct|BreakTimerHandlerEntry (|Copy (Utilities|Array|Get(acopy) _callbacktimers _output_get)))) DeltaSeconds) (.bSetForCallback (Utilities|Struct|BreakTimerHandlerEntry (|Copy (Utilities|Array|Get(acopy) _callbacktimers _output_get)))))))))
            (Development|ExecuteConsoleCommand (Utilities|String|Append "AJBExecInternal Callback " (Utilities|String|ToString(Integer) (LocalVariables|GetCurrentIndex))) (Game|GetPlayerController 0))
            (Development|PrintString (Utilities|String|Append "AJBExecInternal Callback " (Utilities|String|ToString(Integer) (LocalVariables|GetCurrentIndex))) true true "(R=0.128574,G=1.000000,B=0.000000,A=1.000000)" 1e+01)
            (|SetBy-RefVar (Utilities|Array|Get(acopy) (Variables|Default|GetCallbackTimers) (LocalVariables|GetCurrentIndex)) (Utilities|Struct|MakeTimerHandlerEntry (.pAddress (Utilities|Struct|BreakTimerHandlerEntry (|Copy (Utilities|Array|Get(acopy) (Variables|Default|GetCallbackTimers) (LocalVariables|GetCurrentIndex))))) (.fWaitFor (Utilities|Struct|BreakTimerHandlerEntry (|Copy (Utilities|Array|Get(acopy) (Variables|Default|GetCallbackTimers) (LocalVariables|GetCurrentIndex))))) (.fTimeElapsed (Utilities|Struct|BreakTimerHandlerEntry (|Copy (Utilities|Array|Get(acopy) (Variables|Default|GetCallbackTimers) (LocalVariables|GetCurrentIndex))))) true))))))))

(fn BeginInternalTick
  (CallFunction|EventInternalTick))