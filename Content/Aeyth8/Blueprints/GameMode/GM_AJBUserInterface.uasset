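; GM_AJBUserInterface is a Game Mode for the user interface that holds version info and a reference to the current scope widget.
; Setters store both values, and a getter returns the version info as text.
; EventOnTabVersioning appends a versionless option through ExecInternalAppendOp when the widget is valid and the version still equals the placeholder string.
; BeginPlay, Tick and the construction script are empty.
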(event EventBeginPlay)

(event EventTick
  (params (DeltaSeconds :type Float%20%28single-precision%29)))

(fn ConstructionScript)

(fn SetGlobalGameModeScopeVersioningInfo
  (params (NewVersioningInfo :type String))
  (Variables|Default|SetVersioningInfo NewVersioningInfo))

(fn GetVersioningInfo
  (return (Utilities|Text|ToText(String) (Variables|Default|GetVersioningInfo))))

(fn SetCurrentScopeWidget
  (params (InWidget :type User%20Widget%20Object%20Reference))
  (Variables|Default|SetCurrentScopeWidget InWidget))

(fn EventonTabVersioning
  (if (and (Utilities|IsValid (Variables|Default|GetCurrentScopeWidget)) (Utilities|Enum|Equal(Enum) (Variables|Default|GetVersioningInfo) (Utilities|String|MakeLiteralString "VERSION_PLACEHOLDER")))
    (CallFunction|ExecInternalAppendOp "?VERSIONLESS")))