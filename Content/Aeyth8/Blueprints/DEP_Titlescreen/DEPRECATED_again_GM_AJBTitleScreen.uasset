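; Deprecated game mode for an AJB title screen.
; On BeginPlay it shows the mouse cursor and starts the attract background music through an AJBExecInternal console command.
; InitTitleScreenWidget creates the old title screen widget, stores it and adds it to the viewport, with a getter exposing it.
; Nothing in this graph calls that init, and the event graph's guarded create-and-show logic is disconnected.
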(event EventBeginPlay
  (bind _returnvalue (Game|GetPlayerController 0))
  (Variables|/Script/Engine.PlayerController|SetbShowMouseCursor _returnvalue true)
  (Development|ExecuteConsoleCommand "AJBExecInternal PlayBG Sound.BGM.Play.BGM01.Attract" _returnvalue))

(event EventTick
  (params (DeltaSeconds :type Float%20%28single-precision%29)))

(fn ConstructionScript)

(fn GetTitleScreenWidget
  (return (Variables|Default|GetTitleScreenWidget)))

(fn InitTitleScreenWidget
  (bind _returnvalue (UserInterface|CreateWidget "/Game/Aeyth8/Blueprints/UI/TitleScreen/OLD_WBP_AJBTitleScreen.OLD_WBP_AJBTitleScreen_C" (Game|GetPlayerController 0)))
  (bind _output_get (Variables|Default|SetTitleScreenWidget _returnvalue))
  (UserInterface|Viewport|AddtoViewport (stale _output_get) 0))